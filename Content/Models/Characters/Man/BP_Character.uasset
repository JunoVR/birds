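; Configurable male or female character with Wood and Pillow props, whose shirt animation plays at BreathSpeed to set the breathing rate.
; The construction script toggles head and hair via HeadOn, then shows one body's meshes and hides the other's based on IsMale.
; LevelLighting then selects AO or Snow material instances for that body and its props, though the male Wood keeps its AO material in both modes.
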(event EventBeginPlay
  (Components|Timeline|SetPlayRate (Variables|Default|GetMan_Shirt) (Variables|Default|GetBreathSpeed)) ; Sets the Breathing Speed of Animation
)

(event EventActorBeginOverlap
  (params (OtherActor :type Actor%20Object%20Reference)))

(event EventTick
  (params (DeltaSeconds :type Float%20%28single-precision%29)))

(fn ConstructionScript
  (Rendering|SetVisibility (Variables|Default|GetMan_Head) (Variables|Default|GetHeadOn?) false)
  (if (Variables|Default|GetIsMale?) ; Is It Man or Woman?
    (CallFunction|ShowManHideWoman)
    ;[1 1 1] Lighting Type
    (switch int (Variables|Default|GetLevelLighting)
      (:0
        (CallFunction|SetLightingAOMan))
      (:1
        (CallFunction|SetLightingSnowMan)))
    (else
      (CallFunction|HideManShowWoman)
      (switch int (Variables|Default|GetLevelLighting)
        (:0
          (CallFunction|SetLightingAOWoman))
        (:1
          (CallFunction|SetLightingSnowWoman))))))

(fn HideManShowWoman
  (Rendering|SetVisibility (Variables|Default|GetMan_Jeans) false false)
  (Rendering|SetVisibility (Variables|Default|GetWom_Pants) true false)
  (Rendering|Material|SetMaterial (Variables|Default|GetWood) 0 "/Game/Models/Characters/Woman/Occlusion_Lightmaps/Wom_Occ_Wood_Inst.Wom_Occ_Wood_Inst")
  (Rendering|Material|SetMaterial (Variables|Default|GetPillow) 0 "/Game/Models/Characters/Woman/Occlusion_Lightmaps/Wom_AO_Pillow_inst.Wom_AO_Pillow_inst"))

(fn ShowManHideWoman
  (Rendering|SetVisibility (Variables|Default|GetMan_Jeans) true false)
  (Rendering|SetVisibility (Variables|Default|GetWom_Pants) false false)
  (Rendering|Material|SetMaterial (Variables|Default|GetWood) 0 "/Game/Models/Characters/Man/Occlusion_Lightmaps/Wood_AO_Inst.Wood_AO_Inst")
  (Rendering|Material|SetMaterial (Variables|Default|GetPillow) 0 "/Game/Models/Characters/Man/Occlusion_Lightmaps/Pillow_AO_Inst.Pillow_AO_Inst"))

(fn SetLightingAOMan
  (Rendering|Material|SetMaterial (Variables|Default|GetMan_Arm) 0 "/Game/Models/Characters/Man/Occlusion_Lightmaps/Arms_AO_Inst.Arms_AO_Inst")
  (Rendering|Material|SetMaterial (Variables|Default|GetMan_Head) 0 "/Game/Models/Characters/Man/Occlusion_Lightmaps/Head_AO_Inst.Head_AO_Inst")
  (Rendering|Material|SetMaterial (Variables|Default|GetMan_Jeans) 0 "/Game/Models/Characters/Man/Occlusion_Lightmaps/Pants_AO_Inst.Pants_AO_Inst")
  (Rendering|Material|SetMaterial (Variables|Default|GetPillow) 0 "/Game/Models/Characters/Man/Occlusion_Lightmaps/Pillow_AO_Inst.Pillow_AO_Inst")
  (Rendering|Material|SetMaterial (Variables|Default|GetMan_Shirt) 0 "/Game/Models/Characters/Man/Occlusion_Lightmaps/Shirt_AO_Inst.Shirt_AO_Inst")
  (Rendering|Material|SetMaterial (Variables|Default|GetMan_Shoes) 0 "/Game/Models/Characters/Man/Occlusion_Lightmaps/Shoes_AO_Inst.Shoes_AO_Inst"))

(fn SetLightingSnowMan
  (Rendering|Material|SetMaterial (Variables|Default|GetMan_Arm) 0 "/Game/Models/Characters/Man/Snow_Lightmaps/Man_Sn_ArmsInst.Man_Sn_ArmsInst")
  (Rendering|Material|SetMaterial (Variables|Default|GetMan_Head) 0 "/Game/Models/Characters/Man/Snow_Lightmaps/Man_Sn_HeadInst.Man_Sn_HeadInst")
  (Rendering|Material|SetMaterial (Variables|Default|GetMan_Jeans) 0 "/Game/Models/Characters/Man/Snow_Lightmaps/Man_Sn_PantsInst.Man_Sn_PantsInst")
  (Rendering|Material|SetMaterial (Variables|Default|GetPillow) 0 "/Game/Models/Characters/Man/Snow_Lightmaps/Man_Sn_PillowInst.Man_Sn_PillowInst")
  (Rendering|Material|SetMaterial (Variables|Default|GetMan_Shirt) 0 "/Game/Models/Characters/Man/Snow_Lightmaps/Man_Sn_ShirtInst.Man_Sn_ShirtInst")
  (Rendering|Material|SetMaterial (Variables|Default|GetMan_Shoes) 0 "/Game/Models/Characters/Man/Snow_Lightmaps/Man_Sn_ShoesInst.Man_Sn_ShoesInst"))

(fn SetLightingAOWoman
  (Rendering|Material|SetMaterial (Variables|Default|GetWom_Hands_2) 0 "/Game/Models/Characters/Woman/Occlusion_Lightmaps/Wom_AO_Arms.Wom_AO_Arms")
  (Rendering|Material|SetMaterial (Variables|Default|GetWom_Head) 0 "/Game/Models/Characters/Woman/Occlusion_Lightmaps/Wom_AO_Head.Wom_AO_Head")
  (Rendering|Material|SetMaterial (Variables|Default|GetWom_Pants) 0 "/Game/Models/Characters/Woman/Occlusion_Lightmaps/Wom_AO_Pants.Wom_AO_Pants")
  (Rendering|Material|SetMaterial (Variables|Default|GetPillow) 0 "/Game/Models/Characters/Woman/Occlusion_Lightmaps/Wom_AO_Pillow_inst.Wom_AO_Pillow_inst")
  (Rendering|Material|SetMaterial (Variables|Default|GetWom_Shirt) 0 "/Game/Models/Characters/Woman/Occlusion_Lightmaps/Wom_AO_Shirt.Wom_AO_Shirt")
  (Rendering|Material|SetMaterial (Variables|Default|GetWood) 0 "/Game/Models/Characters/Woman/Occlusion_Lightmaps/Wom_Occ_Wood_Inst.Wom_Occ_Wood_Inst"))

(fn SetLightingSnowWoman
  (Rendering|Material|SetMaterial (Variables|Default|GetWom_Hands_2) 0 "/Game/Models/Characters/Woman/Snow_Lightmaps/Wom_Sn_Arms.Wom_Sn_Arms")
  (Rendering|Material|SetMaterial (Variables|Default|GetWom_Head) 0 "/Game/Models/Characters/Woman/Snow_Lightmaps/Wom_Sn_Head.Wom_Sn_Head")
  (Rendering|Material|SetMaterial (Variables|Default|GetWom_Pants) 0 "/Game/Models/Characters/Woman/Snow_Lightmaps/Wom_Sn_Pants.Wom_Sn_Pants")
  (Rendering|Material|SetMaterial (Variables|Default|GetPillow) 0 "/Game/Models/Characters/Woman/Snow_Lightmaps/Wom_Sn_Pillow.Wom_Sn_Pillow")
  (Rendering|Material|SetMaterial (Variables|Default|GetWom_Shirt) 0 "/Game/Models/Characters/Woman/Snow_Lightmaps/Wom_Sn_Shirt.Wom_Sn_Shirt")
  (Rendering|Material|SetMaterial (Variables|Default|GetWood) 0 "/Game/Models/Characters/Woman/Snow_Lightmaps/Wom_Sn_Wood.Wom_Sn_Wood"))