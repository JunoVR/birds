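; Breathing-cycle actor that shows exhale and inhale particle effects oriented to the player camera and broadcasts each breath phase.
; Tick matches both emitters to camera rotation and places the inhale emitter slightly ahead of the root along the view direction.
; StartBreath repeats on a timer, using parallel Sequence delays to toggle the "Shnur" emitters and fire the breath dispatcher for out, hold-out, in and hold-in.
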(event Custom|Start%20Breath
  (Utilities|Time|SetTimerbyEvent (delegate Custom|Start%20Breath) 12.0 true)
  (Utilities|FlowControl|Sequence
    (:then_0
      (Utilities|FlowControl|Delay 2.0)
      (Effects|Components|ParticleSystem|SetEmitterEnable (Variables|Default|GetP_OutBreath) "Shnur" true)
      (Default|CallBreathDispatcher "OutBreath"))
    (:then_1
      (Utilities|FlowControl|Delay 6.0)
      (Effects|Components|ParticleSystem|SetEmitterEnable (Variables|Default|GetP_OutBreath) "Shnur" false)
      (Default|CallBreathDispatcher "HoldOutBreath"))
    (:then_2
      (Utilities|FlowControl|Delay 8.0)
      (Effects|Components|ParticleSystem|SetEmitterEnable (Variables|Default|GetP_InBreath) "Shnur" true)
      (Default|CallBreathDispatcher "InBreath"))
    (:then_3
      (Utilities|FlowControl|Delay 12.0)
      (Effects|Components|ParticleSystem|SetEmitterEnable (Variables|Default|GetP_InBreath) "Shnur" false)
      (Default|CallBreathDispatcher "HoldInBreath"))))

(event EventBeginPlay
  (CallFunction|StartBreath)
  (Effects|Components|ParticleSystem|SetEmitterEnable (Variables|Default|GetP_OutBreath) "Shnur" false)
  (Effects|Components|ParticleSystem|SetEmitterEnable (Variables|Default|GetP_InBreath) "Shnur" false))

(event EventTick
  (params (DeltaSeconds :type Float%20%28single-precision%29))
  ;[1 1 1] Update rotation of In and Our Breath to be relative to cam direction
  (Transformation|SetWorldRotation (Variables|Default|GetP_OutBreath) (Camera|GetCameraRotation (Game|GetPlayerCameraManager 0)) false false)
  (Transformation|SetWorldLocation (Variables|Default|GetP_InBreath) (+ (Transformation|GetWorldLocation (Variables|Default|GetDefaultSceneRoot)) (* (Math|Vector|GetForwardVector (Camera|GetCameraRotation (Game|GetPlayerCameraManager 0))) 4e+01)) false false))

(fn ConstructionScript)