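; Birds Blueprint that changes the speed of a bird particle effect in response to breathing.
; On BeginPlay it binds to the BreathBP breath dispatcher and creates a dynamic material instance on the bird particle system.
; Each breath event sets that material's Speed parameter, higher on the in breath and lower on the out breath.
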(event Custom|BreathEvent
  (params (BreathStage :type String))
  (switch string BreathStage
    (:OutBreath
      (Rendering|Material|SetScalarParameterValue (Variables|Default|GetBirdMaterial) "Speed" 1.5 :!class /Script/Engine.MaterialInstanceDynamic))
    (:InBreath
      (Rendering|Material|SetScalarParameterValue (Variables|Default|GetBirdMaterial) "Speed" 2.5 :!class /Script/Engine.MaterialInstanceDynamic))))

(event EventBeginPlay
  (EventDispatchers|BindEventtoBreathDispatcher (Variables|Default|GetBreathBP) (delegate Custom|BreathEvent))
  (bind _returnvalue (Rendering|Material|CreateDynamicMaterialInstance (Variables|Default|GetBirdParticleSystem) 0 "/Game/Birds/Materials/M_Bird_Particle_Inst.M_Bird_Particle_Inst" :!class /Script/Engine.PrimitiveComponent))
  (Variables|Default|SetBirdMaterial _returnvalue))

(fn ConstructionScript)